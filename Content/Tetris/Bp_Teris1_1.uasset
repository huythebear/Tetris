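; Tetris game manager actor that builds the board from instanced meshes, spawns random pieces with a next-piece preview, and handles input.
; Tick steps the active piece; on landing, its cubes become static mesh components on this actor.
; Line traces across the landed rows detect and destroy full lines, and box traces gather cubes above to shift down.
; Cleared lines drive score, level and fall speed; a blocked spawn point clears the board and opens EndMenu.
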(event Custom|KeyDown
  (params (press? :type Boolean))
  (bind _speedoneticklevel (Variables|Grid|GetSpeedOneTickLevel))
  ;[1 1 1] Key
  (if press?
    (bind _output_get (Variables|Grid|SetSpeedDown (/ _speedoneticklevel 2e+01))) ; Player Click Key Down=More Game Speed
    (Variables|Grid|SetTimeDownNextTick (- (Variables|Grid|GetTimeDownNextTick) _output_get)) ; Update Tick-Time
    (else
      (Variables|Grid|SetSpeedDown _speedoneticklevel) ; Restore Game Speed
    )))

(event Custom|KeyRight
  (params (press? :type Boolean))
  ;[1 1 1] Key
  (Variables|PressKey|SetRight press?))

(event Custom|RestartGameNewGame
  (bind _returnvalue (Game|GetPlayerController 0))
  ;[1 1 1] Restart Game NewGame
  (Variables|/Script/Engine.PlayerController|SetbShowMouseCursor _returnvalue false)
  (Input|SetInputModeGameOnly _returnvalue)
  (Variables|Default|SetScoreGame 0)
  (Utilities|GameScore)
  (Variables|Default|SetLinesGame 0)
  (Utilities|GameLines)
  (Variables|Default|SetLvlGame 2)
  (Utilities|GameLvl)
  (Variables|Default|SetEndGame false)
  (Development|SetHiddeninGame (Variables|Default|GetTextRender_GameOver) true false)
  (Variables|Grid|SetSpeedLeftRight 0.07)
  (bind _output_get (Variables|Grid|SetSpeedOneTickLevel (Variables|Default|GetBaseGameSpeed)))
  (Variables|Grid|SetSpeedDown _output_get)
  (Utilities|FlowControl|Delay 0.2)
  (CallFunction|SpawnBpBlock))

(event Custom|EndGameRemoveAllBlock
  (bind _arrowcentalpointspawnblock (Variables|Default|GetArrowCentalPointSpawnBlock))
  (bind _returnvalue (Transformation|GetWorldLocation _arrowcentalpointspawnblock))
  ;[1 1 1] End Game Remove All Block
  (bind _outhits (Class|KismetSystemLibrary|BoxTraceMultiforObjects (Math|Vector|MakeVector (.x _returnvalue) 0.0 (.z _returnvalue)) (Math|Vector|MakeVector (.x _returnvalue) 0.0 1e+02) (Math|Vector|MakeVector (Math|Conversions|ToFloat(Integer) (/ (* (- (Variables|Default|GetWidth) 2) 100) 2)) 0.0 0.0) "0, 0, 0" (Utilities|Array|MakeArray "ObjectTypeQuery1") false 0 "None" false))
  (for _array_element _outhits
    (Components|DestroyComponent (.HitComponent (Collision|BreakHitResult _array_element)))))

(event Custom|DetectBlockFullLine
  ;[1 1 1] Detect Block Full Line
  (Variables|BlockMaterial|SetDetectBlockgetIndex (+ (Variables|BlockMaterial|GetDetectBlockgetIndex) 1))
  (if (Utilities|Array|IsValidIndex (Variables|BlockMaterial|GetDetectBlockLocationZSort) (Variables|BlockMaterial|GetDetectBlockgetIndex))
    (bind (_outhits _returnvalue) (Class|KismetSystemLibrary|LineTraceMultiforObjects (Math|Vector|MakeVector (Math|Conversions|ToFloat(Integer) (* (- (Variables|Default|GetWidth) 1) 100)) 0.0 (Math|Conversions|ToFloat(Integer) (Utilities|Array|Get(acopy) (Variables|BlockMaterial|GetDetectBlockLocationZSort) (Variables|BlockMaterial|GetDetectBlockgetIndex)))) (Math|Vector|MakeVector 1e+02 0.0 (Math|Conversions|ToFloat(Integer) (Utilities|Array|Get(acopy) (Variables|BlockMaterial|GetDetectBlockLocationZSort) (Variables|BlockMaterial|GetDetectBlockgetIndex)))) (Utilities|Array|MakeArray "ObjectTypeQuery1") false 0 "None" false))
    (if _returnvalue
      (if (== (Utilities|Array|LastIndex _outhits) (- (Variables|Default|GetWidth) 2))
        (Variables|Default|SetScoreGameCounter (+ (Variables|Default|GetScoreGameCounter) 1))
        (for _array_element _outhits
          (Components|DestroyComponent (.HitComponent (Collision|BreakHitResult _array_element))))
        (CallFunction|AllBlockOneDegreeDown)
        (else
          (CallFunction|DetectBlockFullLine :!label _label)))
      (else
        (goto _label)))
    (else
      (if (== (Variables|Default|GetScoreGameCounter) 0)
        _
        (else
          (Variables|Default|SetScoreGame (+ (Variables|Default|GetScoreGame) (* (Math|Integer|Clamp(Integer) (+ (Variables|Default|GetScoreGameCounter) (- (Variables|Default|GetScoreGameCounter) 1)) 0 99) (- (Variables|Default|GetWidth) 1))))
          (Utilities|GameScore)
          (Variables|Default|SetLinesGame (+ (Variables|Default|GetLinesGame) (Variables|Default|GetScoreGameCounter)))
          (Utilities|GameLines)
          (Variables|Default|SetLvlGame (/ (Variables|Default|GetLinesGame) 10))
          (if (> (Variables|Default|GetLvlGame) (Variables|Default|GetLvlGame_0))
            (Variables|Default|SetLvlGame_0 (Variables|Default|GetLvlGame))
            (Utilities|GameLvl)
            (Variables|Grid|SetSpeedOneTickLevel (- (Variables|Default|GetBaseGameSpeed) (* (Math|Conversions|ToFloat(Integer) (Variables|Default|GetLvlGame)) 0.03)))
            (Variables|Grid|SetSpeedDown (Variables|Grid|GetSpeedOneTickLevel)) ; Restore Game Speed
          )))
      (CallFunction|SpawnBpBlock))))

(event Custom|KeyLeft
  (params (press? :type Boolean))
  ;[1 1 1] Key
  (Variables|PressKey|SetLeft press?))

(event Custom|AllBlockOneDegreeDown
  (bind _arrowcentalpointspawnblock (Variables|Default|GetArrowCentalPointSpawnBlock))
  (bind _returnvalue (Transformation|GetWorldLocation _arrowcentalpointspawnblock))
  ;[1 1 1] All Block One Degree Down
  (Utilities|Array|Clear (Variables|Default|GetBlockOneDegreeDown))
  (Variables|BlockMaterial|SetBlockDownCounter 0)
  (bind (_outhits _returnvalue_2) (Class|KismetSystemLibrary|BoxTraceMultiforObjects (Math|Vector|MakeVector (.x _returnvalue) 0.0 (.z _returnvalue)) (Math|Vector|MakeVector (.x _returnvalue) 0.0 (Math|Conversions|ToFloat(Integer) (Utilities|Array|Get(acopy) (Variables|BlockMaterial|GetDetectBlockLocationZSort) (Variables|BlockMaterial|GetDetectBlockgetIndex)))) (Math|Vector|MakeVector (Math|Conversions|ToFloat(Integer) (/ (* (- (Variables|Default|GetWidth) 2) 100) 2)) 0.0 0.0) "0, 0, 0" (Utilities|Array|MakeArray "ObjectTypeQuery1") false 0 "None" false))
  (if _returnvalue_2
    (for _array_element _outhits
      (Utilities|Array|Add (Variables|Default|GetBlockOneDegreeDown) (.HitComponent (Collision|BreakHitResult _array_element))))
    (Utilities|FlowControl|Delay 0.01 :!label _label)
    (bind _output_get (Variables|BlockMaterial|SetBlockDownCounter (+ (Variables|BlockMaterial|GetBlockDownCounter) 1)))
    (if (> _output_get 2)
      (CallFunction|DetectBlockFullLine)
      (else
        (for _array_element_2 (Variables|Default|GetBlockOneDegreeDown)
          (Transformation|SetWorldLocation _array_element_2 (- (Transformation|GetWorldLocation _array_element_2) "0, 0,50.000000") false false))
        (goto _label)))
    (else
      (Utilities|FlowControl|Delay 0.02)
      (CallFunction|DetectBlockFullLine))))

(event Custom|KeyUp
  (params (press? :type Boolean))
  ;[1 1 1] Key
  (if press?
    (Default|Blockrotation (Variables|Default|GetRef_BpBlock))))

(event Custom|BlockSortLocation
  (bind _detectblocklocationz (Variables|BlockMaterial|GetDetectBlockLocationZ))
  (bind _detectblocklocationz_2 (Variables|BlockMaterial|GetDetectBlockLocationZ))
  (bind (_indexofmaxvalue _maxvalue) (Math|Integer|MaxOfIntArray _detectblocklocationz_2))
  ;[1 1 1] Block Sort Location
  (Utilities|Array|Clear (Variables|BlockMaterial|GetDetectBlockLocationZSort))
  (Utilities|Array|Clear (Variables|BlockMaterial|GetDetectBlockLocationZ))
  (for (_array_element _array_index) (Variables|/Game/Tetris/Bp_Block.Bp_Block_C|GetAllBlock (Variables|Default|GetRef_BpBlock))
    (if (== _array_index 0)
      (Utilities|Array|Add (Variables|BlockMaterial|GetDetectBlockLocationZ) (Math|Float|Truncate (.z (Transformation|GetWorldLocation _array_element))) :!label _label)
      (elif (== (Utilities|Array|FindItem (Variables|BlockMaterial|GetDetectBlockLocationZ) (Math|Float|Truncate (.z (Transformation|GetWorldLocation _array_element)))) -1)
        (goto _label))))
  (Utilities|Array|Add (Variables|BlockMaterial|GetDetectBlockLocationZSort) _maxvalue :!label _label_2)
  (Utilities|Array|RemoveIndex _detectblocklocationz _indexofmaxvalue)
  (if (Utilities|Array|IsValidIndex _detectblocklocationz)
    (goto _label_2)
    (else
      (Variables|BlockMaterial|SetDetectBlockgetIndex -1)
      (CallFunction|DetectBlockFullLine))))

(event Custom|EventAddStaticMesh
  ;[1 1 1] Event Add Static Mesh
  (for _array_element (Variables|/Game/Tetris/Bp_Block.Bp_Block_C|GetAllBlock (Variables|Default|GetRef_BpBlock))
    (bind _returnvalue (AddComponent|AddStaticMeshComponent false (Math|Transform|MakeTransform (Transformation|GetWorldLocation _array_element) "0, 0, 0" "1,1,1"))) ; World Location
    (Components|StaticMesh|SetStaticMesh _returnvalue (Variables|/Script/Engine.StaticMeshComponent|GetStaticMesh _array_element))
    (Rendering|Material|SetMaterial _returnvalue 0 (Rendering|Material|GetMaterial _array_element 0))))

(event Custom|SpawnBpBlock
  ;[1 1 1] Spawn Bp Block
  (bind _ref_bpblock (Variables|Default|GetRef_BpBlock)
    (:then
      (CallFunction|CheckEndGame)
      (Actor|DestroyActor _ref_bpblock))
    (:else
      _))
  (if (Variables|Default|GetEndGame)
    (CallFunction|EndGameRemoveAllBlock)
    (CallFunction|RestartGameNewGame)
    (bind _returnvalue (UserInterface|CreateWidget "/Game/Player/EndMenu.EndMenu_C"))
    (UserInterface|Viewport|AddtoViewport _returnvalue 0)
    (Variables|/Script/Engine.PlayerController|SetbShowMouseCursor (Game|GetPlayerController 0) true)
    (else
      (Variables|Default|GetRef_BpBlock_Next_Block
        (:then
          (bind _output_get (Variables|Default|SetRef_BpBlock (Variables|Default|GetRef_BpBlock_Next_Block) :!label _label))
          (Transformation|SetActorLocation _output_get (Transformation|GetWorldLocation (Variables|Default|GetArrowCentalPointSpawnBlock)) false false)
          (Rendering|SetActorHiddenInGame _output_get false)
          (Utilities|FlowControl|Sequence
            (:then_0
              (bind _returnvalue_2 (Game|SpawnActorfromClass (Utilities|Array|Get(acopy) (Variables|Default|GetAllBlocks) (Math|Random|RandomIntegerinRange 0 6)) (Math|Transform|MakeTransform (Transformation|GetWorldLocation (Variables|Default|GetArrow_SpawnNextBlock)) "0, 0, 0" "1,1,1") "Undefined" 0 0 :!label _label_2))
              (bind _asbp_block (Utilities|Casting|CastToBp_Block _returnvalue_2))
              (bind _output_get_2 (Variables|Default|SetRef_BpBlock_Next_Block _asbp_block))
              (Rendering|SetActorHiddenInGame _output_get_2 true)
              (Variables|BlockMaterial|SetBlockNumberColor (Math|Random|RandomIntegerinRange 0 (Utilities|Array|LastIndex (Variables|BlockMaterial|GetAllBlockMaterial))))
              (Rendering|Material|SetMaterial (Variables|/Game/Tetris/Bp_Block.Bp_Block_C|GetAllBlock (Variables|Default|GetRef_BpBlock_Next_Block)) 0 (Utilities|Array|Get(acopy) (Variables|BlockMaterial|GetAllBlockMaterial) (Variables|BlockMaterial|GetBlockNumberColor)))
              (Rendering|SetActorHiddenInGame (Variables|Default|GetRef_BpBlock_Next_Block) false))
            (:then_1
              (Utilities|FlowControl|Delay 0.01)
              (Actor|Tick|SetActorTickEnabled true))))
        (:else
          (Utilities|FlowControl|Sequence
            (:then_0
              (goto _label_2))
            (:then_1
              (goto _label))))))))

(event Custom|CheckEndGame
  (bind _arrowcentalpointspawnblock (Variables|Default|GetArrowCentalPointSpawnBlock))
  (bind _returnvalue (Transformation|GetWorldLocation _arrowcentalpointspawnblock))
  ;[1 1 1] Check End Game
  (if (Math|Vector|Equal(Vector) _returnvalue (Transformation|GetWorldLocation (Variables|/Game/Tetris/Bp_Block.Bp_Block_C|GetSm_Center (Variables|Default|GetRef_BpBlock))) 2.0)
    (bind _returnvalue_2 (Class|KismetSystemLibrary|BoxTraceSingleforObjects _returnvalue (+ _returnvalue "0, 0,1.000000") "45.000000,20.000000,45.000000" "0, 0, 0" (Utilities|Array|MakeArray "ObjectTypeQuery1") false 0 "None" false))
    (Variables|Default|SetEndGame _returnvalue_2)))

(event EventBeginPlay
  ;[1 1 1] Key
  (CallFunction|RestartGameNewGame))

(event EventTick
  (params (DeltaSeconds :type Float%20%28single-precision%29))
  (bind _returnvalue (Utilities|Time|GetGameTimeinSeconds))
  ;[1 1 1] Event Tick
  (Utilities|FlowControl|Sequence
    (:then_0
      (if (>= _returnvalue (Variables|Grid|GetTimeDownNextTick))
        (Variables|Grid|SetTimeDownNextTick (+ (Variables|Grid|GetSpeedDown) _returnvalue))
        (bind _collison_ (Default|DetectClollison (Variables|Default|GetRef_BpBlock) false true false))
        (if _collison_
          (Actor|Tick|SetActorTickEnabled false)
          (Variables|Default|SetScoreGameCounter 0)
          (Rendering|SetActorHiddenInGame (Variables|Default|GetRef_BpBlock) true)
          (CallFunction|EventAddStaticMesh)
          (CallFunction|BlockSortLocation)
          (else
            (CallFunction|NextBlockLocation)))))
    (:then_1
      (if (>= _returnvalue (Variables|Grid|GetSpeedLeftRightNexttick))
        (Variables|Grid|SetSpeedLeftRightNexttick 0.0)
        (if (Variables|PressKey|GetLeft)
          (bind _collison__2 (Default|DetectClollison (Variables|Default|GetRef_BpBlock) false false true))
          (if (not _collison__2)
            (CallFunction|NextBlockLocation 1))
          (elif (Variables|PressKey|GetRight)
            (bind _collison__3 (Default|DetectClollison (Variables|Default|GetRef_BpBlock) false false false))
            (if (not _collison__3)
              (CallFunction|NextBlockLocation 2))))))))

(fn ConstructionScript
  (bind _returnvalue (Transformation|GetActorLocation))
  (bind _returnvalue_2 (Transformation|GetActorLocation))
  (bind _width (Variables|Default|GetWidth))
  (bind _height (Variables|Default|GetHeight))
  (bind _width_2 (Variables|Default|GetWidth))
  (bind _returnvalue_3 (- _height 1))
  (bind (_x _y _z) (Math|Vector|BreakVector _returnvalue))
  (bind _y_2 (Math|Vector|BreakVector _returnvalue_2))
  (bind _returnvalue_4 (/ _width 2))
  (bind _returnvalue_5 (* _width_2 100))
  (bind _returnvalue_6 (+ _returnvalue_5 320))
  (bind _returnvalue_7 (* _returnvalue_3 100))
  (bind _returnvalue_8 (+ _y_2 6e+02))
  (bind _returnvalue_9 (+ _z 9e+02))
  (bind _returnvalue_10 (+ _y 5e+01))
  (bind _returnvalue_11 (* _returnvalue_4 100))
  (bind _returnvalue_12 (Math|Conversions|ToFloat(Integer) _returnvalue_6))
  (bind _returnvalue_13 (/ _returnvalue_7 2))
  (bind _returnvalue_14 (Math|Conversions|ToFloat(Integer) _returnvalue_11))
  (bind _returnvalue_15 (- _returnvalue_9 3e+02))
  (bind _returnvalue_16 (Math|Conversions|ToFloat(Integer) _returnvalue_13))
  (Transformation|SetRelativeLocation (Variables|Default|GetArrowCentalPointSpawnBlock) (Math|Vector|MakeVector _returnvalue_14 0.0 (Math|Conversions|ToFloat(Integer) _returnvalue_7)) false false)
  (Transformation|SetRelativeLocation (Variables|Default|GetArrow_SpawnNextBlock) (Math|Vector|MakeVector (Math|Conversions|ToFloat(Integer) (+ (* (Variables|Default|GetWidth) 100) 350)) 0.0 (Math|Conversions|ToFloat(Integer) (- _returnvalue_7 100))) false false)
  (Transformation|SetWorldLocation (Variables|Default|GetTextRender_GameOver) (Math|Vector|MakeVector _returnvalue_14 _returnvalue_8 _returnvalue_16) false false)
  (Transformation|SetWorldLocation (Variables|Default|GetTextRender_GameOverCounter) (Math|Vector|MakeVector _returnvalue_14 _returnvalue_8 (- _returnvalue_16 1.5e+02)) false false)
  (Transformation|SetWorldLocation (Variables|Default|GetTextRender_Score) (Math|Vector|MakeVector _returnvalue_12 _returnvalue_10 _returnvalue_9) false false)
  (Transformation|SetWorldLocation (Variables|Default|GetTextRender_Lines) (Math|Vector|MakeVector _returnvalue_12 _returnvalue_10 _returnvalue_15) false false)
  (Transformation|SetWorldLocation (Variables|Default|GetTextRender_Lvl) (Math|Vector|MakeVector _returnvalue_12 _returnvalue_10 (- _returnvalue_15 3e+02)) false false)
  (for _index (range 0 (Variables|Default|GetWidth))
    (for _index_2 (range 0 (Variables|Default|GetHeight))
      (Components|InstancedStaticMesh|AddInstance (Variables|Default|GetHierarchicalInstancedStaticMesh) (Math|Transform|MakeTransform (Math|Vector|MakeVector (Math|Conversions|ToFloat(Integer) (* _index 100)) (Math|Float|SelectFloat 0.0 -9e+01 (Math|Boolean|ORBoolean (== _index 0) (== _index (Variables|Default|GetWidth)) (== _index_2 0) (== _index_2 (Variables|Default|GetHeight)))) (Math|Conversions|ToFloat(Integer) (* _index_2 100))))))))

(fn NextBlockLocation
  (params (Selection :type Integer))
  (switch int Selection
    (:0
      (LocalVariables|SetL_Location "0, 0,100.000000") ; Down
    )
    (:1
      (LocalVariables|SetL_Location "100.000000, 0, 0") ; Right
    )
    (:2
      (LocalVariables|SetL_Location "-100.000000, 0, 0") ; Left
    ))
  (Transformation|SetActorLocation (Variables|Default|GetRef_BpBlock) (- (Transformation|GetActorLocation (Variables|Default|GetRef_BpBlock)) (LocalVariables|GetL_Location)) false false))